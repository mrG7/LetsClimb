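; Post-process effect actor that plays a "wet bulbs" screen effect when PlayBulbs is called.
; BeginPlay creates a dynamic material instance and adds it to the WetBulbsPostProcess component at zero weight.
; PlayBulbs sets the weight to full and starts two timelines driving the material's blur (scaled by BlurAmount) and distort parameters.
; The distort timeline's finish re-applies full weight, so the blendable is never switched off here.
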(event Custom|PlayBulbs
  (bind _wetbulbsmaterial (Variables|Default|GetWetBulbsMaterial))
  (bind _wetbulbspostprocess (Variables|Default|GetWetBulbsPostProcess))
  (Rendering|AddorUpdateBlendable _wetbulbspostprocess _wetbulbsmaterial 1.0 :!class /Script/Engine.PostProcessVolume)
  (Utilities|IsValid _wetbulbsmaterial
    (:Is%20Valid
      (Utilities|FlowControl|Sequence
        (:then_0
          (bind _blur (Timeline|Timeline_0 PlayFromStart)
            (:Update
              (Rendering|Material|SetScalarParameterValue _wetbulbsmaterial "blur" (* _blur (Variables|Default|GetBlurAmount)) :!class /Script/Engine.MaterialInstanceDynamic))))
        (:then_1
          (bind _distort (Timeline|Timeline_1 PlayFromStart)
            (:Update
              (Rendering|Material|SetScalarParameterValue _wetbulbsmaterial "distort" _distort :!class /Script/Engine.MaterialInstanceDynamic))
            (:Finished
              (Rendering|AddorUpdateBlendable _wetbulbspostprocess _wetbulbsmaterial 1.0 :!class /Script/Engine.PostProcessVolume))))))))

(event EventBeginPlay
  (bind _returnvalue (Rendering|Material|CreateDynamicMaterialInstance "/Game/FX/pp_wetbulbs_Inst.pp_wetbulbs_Inst" :!class /Script/Engine.KismetMaterialLibrary))
  (Variables|Default|SetWetBulbsMaterial _returnvalue)
  (Rendering|AddorUpdateBlendable (Variables|Default|GetWetBulbsPostProcess) (Variables|Default|GetWetBulbsMaterial) 0.0 :!class /Script/Engine.PostProcessVolume))

(event EventActorBeginOverlap
  (params (OtherActor :type Actor%20Object%20Reference)))

(event EventTick
  (params (DeltaSeconds :type Float%20%28single-precision%29)))

(fn ConstructionScript)