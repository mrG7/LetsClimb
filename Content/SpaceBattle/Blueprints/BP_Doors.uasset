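; Sliding door actor that a MyCharacterStar opens through DoAction, with the box trigger telling the character when it enters or leaves the door zone.
; DoAction unlocks linked LockPanels and plays a timeline that moves the mesh, ignoring calls while moving.
; Leaving the box reverses the timeline with audio, relocking panels once closed.
; The construction script applies mesh, sound and box overrides only when OverrideMesh is valid.
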(event OnComponentBeginOverlap(Box)
  (params (OverlappedComponent :type Primitive%20Component%20Object%20Reference) (OtherActor :type Actor%20Object%20Reference) (OtherComp :type Primitive%20Component%20Object%20Reference) (OtherBodyIndex :type Integer) (bFromSweep :type Boolean) (SweepResult :type Hit%20Result%20Structure%20%28by%20ref%29))
  (bind _asmy_character_star (Utilities|Casting|CastToMyCharacterStar OtherActor))
  (Default|OnDoorZoneEnteredEvent _asmy_character_star self))

(event OnComponentEndOverlap(Box)
  (params (OverlappedComponent :type Primitive%20Component%20Object%20Reference) (OtherActor :type Actor%20Object%20Reference) (OtherComp :type Primitive%20Component%20Object%20Reference) (OtherBodyIndex :type Integer))
  (bind _asmy_character_star (Utilities|Casting|CastToMyCharacterStar OtherActor))
  (Default|OnDoorZoneLeavedEvent _asmy_character_star)
  (Audio|Components|Audio|Play (Variables|Default|GetAudio) 0.0)
  (bind (_direction _position) (Timeline|Open%20Doors%20Timeline Reverse)
    (:Update
      (Transformation|SetRelativeLocation (Variables|Default|GetDoorMesh) _position false false)
      (Variables|Default|SetIsDoorInMove true))
    (:Finished
      (Audio|Components|Audio|Stop (Variables|Default|GetAudio))
      (Variables|Default|SetIsDoorInMove false)
      (switch Utilities|FlowControl|Switch|SwitchonETimelineDirection _direction
        (:Backward
          (for _array_element (Variables|Setup|GetLock%20Panels)
            (Utilities|IsValid _array_element
              (:Is%20Valid
                (Default|SetLocked _array_element true)))))))))

(event EventDoAction
  (params (Player :type My%20Character%20Star%20Object%20Reference))
  (if (not (Variables|Default|GetIsDoorInMove))
    (Default|OnDoorZoneLeavedEvent Player)
    (Audio|Components|Audio|Play (Variables|Default|GetAudio) 0.0)
    (for _array_element (Variables|Setup|GetLock%20Panels)
      (Utilities|IsValid _array_element
        (:Is%20Valid
          (Default|SetLocked _array_element false))))
    (bind (_direction _position) (Timeline|Open%20Doors%20Timeline Play)
      (:Update
        (Transformation|SetRelativeLocation (Variables|Default|GetDoorMesh) _position false false)
        (Variables|Default|SetIsDoorInMove true))
      (:Finished
        (Audio|Components|Audio|Stop (Variables|Default|GetAudio))
        (Variables|Default|SetIsDoorInMove false)
        (switch Utilities|FlowControl|Switch|SwitchonETimelineDirection _direction
          (:Backward
            (for _array_element_2 (Variables|Setup|GetLock%20Panels)
              (Utilities|IsValid _array_element_2
                (:Is%20Valid
                  (Default|SetLocked _array_element_2 true))))))))))

(event EventBeginPlay)

(event EventActorBeginOverlap
  (params (OtherActor :type Actor%20Object%20Reference)))

(event EventTick
  (params (DeltaSeconds :type Float%20%28single-precision%29)))

(fn ConstructionScript
  (bind _box (Variables|Default|GetBox))
  (Utilities|IsValid (Variables|Setup|GetOverride%20Mesh)
    (:Is%20Valid
      (Components|StaticMesh|SetStaticMesh (Variables|Default|GetDoorMesh) (Variables|Setup|GetOverride%20Mesh))
      (Audio|Components|Audio|SetSound (Variables|Default|GetAudio) (Variables|Audio|GetOpen%20Sound))
      (Components|Box|SetBoxExtent _box (Variables|Default|GetCollisionBoxSize) true)
      (Transformation|SetRelativeLocation _box (Variables|Default|GetCollisionBoxRelativeLocation) false false))))