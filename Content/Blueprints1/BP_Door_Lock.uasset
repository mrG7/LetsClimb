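; BP_Door_Lock is a door lock whose material visually transitions between locked and unlocked states.
; On BeginPlay it creates a dynamic material instance from slot 3 of its static mesh and applies it back to that slot.
; SetLocked plays a timeline forward to unlock or in reverse to lock, with the timeline driving the material's Lock scalar parameter.
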(event Custom|Set%20Locked
  (params (IsLocked :type Boolean))
  (if IsLocked
    (bind _lock (Timeline|Lock%20Timeline Reverse)
      (:Update
        (Rendering|Material|SetScalarParameterValue (Variables|Default|GetLock%20MID) "Lock" _lock :!class /Script/Engine.MaterialInstanceDynamic)))
    (else
      (Timeline|Lock%20Timeline Play))))

(event EventBeginPlay
  (bind _returnvalue (Rendering|Material|CreateDynamicMaterialInstance (Rendering|Material|GetMaterial (Variables|Debug|GetStaticMeshComponent) 3) :!class /Script/Engine.KismetMaterialLibrary))
  (bind _output_get (Variables|Default|SetLock%20MID _returnvalue))
  (Rendering|Material|SetMaterial (Variables|Debug|GetStaticMeshComponent) 3 _output_get))

(event EventActorBeginOverlap
  (params (OtherActor :type Actor%20Object%20Reference)))

(event EventTick
  (params (DeltaSeconds :type Float%20%28single-precision%29)))

(fn ConstructionScript)