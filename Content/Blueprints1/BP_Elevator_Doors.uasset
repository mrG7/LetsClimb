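; BP_Elevator_Doors is an elevator door actor with two hinged panels that swing open when the player character approaches.
; Entering the Box trigger as MyCharacter waits a short delay, then plays the DoorAnim timeline, which rotates the Left and Right meshes in opposite yaw directions.
; Leaving the box reverses the timeline to close them, and a CloseDoors event lets other logic trigger the same closing.
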(event OnComponentBeginOverlap(Box)
  (params (OverlappedComponent :type Primitive%20Component%20Object%20Reference) (OtherActor :type Actor%20Object%20Reference) (OtherComp :type Primitive%20Component%20Object%20Reference) (OtherBodyIndex :type Integer) (bFromSweep :type Boolean) (SweepResult :type Hit%20Result%20Structure%20%28by%20ref%29))
  (Utilities|Casting|CastToMyCharacter OtherActor)
  (Utilities|FlowControl|Delay 1.0)
  (bind _rotation (Timeline|Door%20Anim Play)
    (:Update
      (Transformation|SetRelativeRotation (Variables|Default|GetLeft) (Math|Rotator|MakeRotator 0.0 0.0 (+ -9e+01 (* _rotation -1.0))) false false)
      (Transformation|SetRelativeRotation (Variables|Default|GetRight) (Math|Rotator|MakeRotator 0.0 0.0 (+ 9e+01 _rotation)) false false))))

(event OnComponentEndOverlap(Box)
  (params (OverlappedComponent :type Primitive%20Component%20Object%20Reference) (OtherActor :type Actor%20Object%20Reference) (OtherComp :type Primitive%20Component%20Object%20Reference) (OtherBodyIndex :type Integer))
  (Utilities|Casting|CastToMyCharacter OtherActor)
  (bind _rotation (Timeline|Door%20Anim Reverse)
    (:Update
      (Transformation|SetRelativeRotation (Variables|Default|GetLeft) (Math|Rotator|MakeRotator 0.0 0.0 (+ -9e+01 (* _rotation -1.0))) false false)
      (Transformation|SetRelativeRotation (Variables|Default|GetRight) (Math|Rotator|MakeRotator 0.0 0.0 (+ 9e+01 _rotation)) false false))))

(event Custom|Close%20Doors
  (bind _rotation (Timeline|Door%20Anim Reverse)
    (:Update
      (Transformation|SetRelativeRotation (Variables|Default|GetLeft) (Math|Rotator|MakeRotator 0.0 0.0 (+ -9e+01 (* _rotation -1.0))) false false)
      (Transformation|SetRelativeRotation (Variables|Default|GetRight) (Math|Rotator|MakeRotator 0.0 0.0 (+ 9e+01 _rotation)) false false))))

(event EventBeginPlay)

(event EventActorBeginOverlap
  (params (OtherActor :type Actor%20Object%20Reference)))

(event EventTick
  (params (DeltaSeconds :type Float%20%28single-precision%29)))

(fn ConstructionScript)