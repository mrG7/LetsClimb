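; SnowArcticPawn is a pawn Blueprint with no active behavior, as its events and construction script are empty.
; The event graph holds disconnected leftovers: zeroed pitch and yaw controller input calls beside empty MouseX and MouseY events.
; An unwired SetWorldLocationAndRotation uses VInterpTo and RInterpTo on player camera manager transforms, resembling an unfinished smoothed camera follow.
; None of this logic runs.
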(event EventBeginPlay)

(event Collision|EventActorBeginOverlap
  (params (OtherActor :type Actor%20Object%20Reference)))

(event EventTick
  (params (DeltaSeconds :type Float%20%28single-precision%29)))

(event Input|MouseEvents|MouseX
  (params (AxisValue :type Float%20%28single-precision%29)))

(event Input|MouseEvents|MouseY
  (params (AxisValue :type Float%20%28single-precision%29)))

(fn ConstructionScript)